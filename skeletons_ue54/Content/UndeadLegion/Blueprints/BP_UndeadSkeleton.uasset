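; Undead skeleton actor with modular armor, tintable socketed eyes, swappable hand-weapon loadouts and a working bow.
; Armor modules follow the body via leader pose, while loadouts spawn socketed weapons and drive grip and finger targets in the AnimBP.
; Clips play as dynamic slot montages for loops, actions and hit overlays, with optional timed startup actions.
; Tick bends the poseable bow and string from right-hand position while attached; release spawns an arrow.
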(event `self.ReceiveBeginPlay`
  (`self.EquipLoadout` (`self.StartLoadout`))
  (`self.PlayLoop` (`self.StartClip`))
  (`self.SetClipHold` (`self.StartHoldLeft`))
  (set `self.StartActionIndex` 0)
  (if (> (`KismetArrayLibrary.Array_Length` (`self.StartActions`)) 0)
    (`KismetSystemLibrary.K2_SetTimer` self "NextStartAction" (`self.StartActionDelay`))))

(event `self.ReceiveEndPlay`
  (params (EndPlayReason :type "EEndPlayReason Enum" :default "Destroyed"))
  (for _array_element (`self.WeaponActors`)
    (`self.K2_DestroyActor` _array_element))
  (`KismetArrayLibrary.Array_Clear` (`self.WeaponActors`)))

(event `self.ReceiveTick`
  (params (DeltaSeconds :type "Float (single-precision)"))
  (if (`self.HasBow`)
    (`/Engine/EditorBlueprintResources/StandardMacros.IsValid` (`self.BowMesh`)
      (:`Is Valid`
        (`self.UpdateBow` DeltaSeconds)))))

(fn `AddModuleComponent`
  (params (Module :type "SkeletalMesh Object Reference"))
  (bind _mesh (`self.Mesh`))
  (bind _returnvalue (`|AddComponentByClass` "/Script/Engine.SkeletalMeshComponent"))
  (`SkeletalMeshComponent.SetSkeletalMeshAsset` _returnvalue Module)
  (`SceneComponent.K2_AttachToComponent` _returnvalue _mesh "None" "SnapToTarget" "SnapToTarget" "SnapToTarget" false)
  (`SkinnedMeshComponent.SetLeaderPoseComponent` _returnvalue _mesh false false)
  (`KismetArrayLibrary.Array_Add` (`self.ArmorComponents`) _returnvalue))

(fn `ApplyDefaultModules`
  (for _array_element (`self.ArmorComponents`)
    (`ActorComponent.K2_DestroyComponent` _array_element))
  (`KismetArrayLibrary.Array_Clear` (`self.ArmorComponents`))
  (for _array_element_2 (`self.DefaultModules`)
    (`self.AddModuleComponent` _array_element_2))
  (`self.ApplyEyes`))

(fn `ApplyEyes`
  (bind _mesh (`self.Mesh`))
  (`SceneComponent.K2_AttachToComponent` (`self.EyeL`) _mesh "EyeL" "SnapToTarget" "SnapToTarget" "KeepRelative" false)
  (`SceneComponent.K2_AttachToComponent` (`self.EyeR`) _mesh "EyeR" "SnapToTarget" "SnapToTarget" "KeepRelative" false)
  (`self.ShowEyes` (`self.EyesVisible`))
  (`self.TintEyes` (`self.EyeColor`)))

(fn `BowAttach`
  (if (`self.HasBow`)
    (`self.BowDraw`)
    (set `self.BowAttached` true)))

(fn `BowDraw`
  (if (`self.HasBow`)
    (`/Engine/EditorBlueprintResources/StandardMacros.IsValid` (`self.HeldArrow`)
      (:`Is Valid`
        (`self.SetActorHiddenInGame` (`self.HeldArrow`) false)))))

(fn `BowRelease`
  (if (and (`self.HasBow`) (`self.BowAttached`))
    (set `self.BowAttached` false)
    (`/Engine/EditorBlueprintResources/StandardMacros.IsValid` (`self.HeldArrow`)
      (:`Is Valid`
        (bind _asstatic_mesh_component (cast `StaticMeshComponent` (`self.GetComponentByClass` (`self.HeldArrow`) "/Script/Engine.StaticMeshComponent")))
        (`|SpawnActorFromClass` (`self.ArrowClass`) (`KismetMathLibrary.MakeTransform` (`SceneComponent.GetSocketLocation` _asstatic_mesh_component "None") (`self.K2_GetActorRotation`)) "AlwaysSpawn" "SelectDefaultAtRuntime" null null)
        (`self.SetActorHiddenInGame` (`self.HeldArrow`) true)))))

(fn `BowReset`
  (set `self.BowAttached` false)
  (set `self.Draw` 0.0)
  (set `self.Apex` (`KismetMathLibrary.MakeVector` 0.0))
  (`/Engine/EditorBlueprintResources/StandardMacros.IsValid` (`self.HeldArrow`)
    (:`Is Valid`
      (`self.SetActorHiddenInGame` (`self.HeldArrow`) true))))

(fn `EquipLoadout`
  (params (Index :type Integer))
  (set `self.BowShotActive` false)
  (`self.BowReset`)
  (for _array_element (`self.WeaponActors`)
    (`self.K2_DestroyActor` _array_element))
  (`KismetArrayLibrary.Array_Clear` (`self.WeaponActors`))
  (set `self.HasWeaponLeft` false)
  (set `self.HasWeaponRight` false)
  (set `self.CurrentLoadout` Index)
  (`|ExecutionSequence`
    (:`then_0`
      (if (`KismetArrayLibrary.Array_IsValidIndex` (`self.LoadoutRight`) Index)
        (`self.SpawnWeapon` Index)
        (`self.SpawnWeapon` Index true)))
    (:`then_1`
      (`self.FindBow`)
      (`self.BowReset`)
      (`self.UpdateHands`))))

(fn `FindBow`
  (set `self.HasBow` false)
  (for _array_element (`self.WeaponActors`)
    (bind _asposeable_mesh_component (cast `PoseableMeshComponent` (`self.GetComponentByClass` _array_element "/Script/Engine.PoseableMeshComponent"))
      (:`then`
        (set `self.BowMesh` _asposeable_mesh_component)
        (set `self.HasBow` true))
      (:`CastFailed`
        (bind _asbp_weapon_arrow (cast `/Game/UndeadLegion/Weapons/Blueprints/BP_Weapon_Arrow` _array_element))
        (set `self.HeldArrow` _asbp_weapon_arrow)))))

(fn `GetFingerIdle`
  (params (Left :type Boolean))
  (returns (On :type Boolean))
  (return (select `bool` Left :`false` (`self.FingerIdleRight`) :`true` (`self.FingerIdleLeft`))))

(fn `GetLoadout`
  (returns (Index :type Integer))
  (return (`self.CurrentLoadout`)))

(fn `IsModuleWorn`
  (params (Module :type "SkeletalMesh Object Reference"))
  (returns (Worn :type Boolean))
  (for _array_element (`self.ArmorComponents`)
    (if (and (== (`SkeletalMeshComponent.GetSkeletalMeshAsset` _array_element) Module) (`SceneComponent.IsVisible` _array_element))
      (return true)))
  (return false))

(fn `NextStartAction`
  (bind _startactionindex (`self.StartActionIndex`))
  (if (`KismetArrayLibrary.Array_IsValidIndex` (`self.StartActions`) _startactionindex)
    (bind _length (`self.PlayAction` (`|GetArrayItem` (`self.StartActions`) _startactionindex) "DefaultSlot" 0.15 0.25 1.0))
    (`KismetSystemLibrary.PrintString` (`KismetStringLibrary.Concat_StrStr` "StartAction " (`KismetStringLibrary.Conv_IntToString` _startactionindex)) false)
    (set `self.StartActionIndex` (+ _startactionindex 1))
    (`KismetSystemLibrary.K2_SetTimer` self "NextStartAction" (+ _length (`self.StartActionGap`)))))

(fn `PauseActions`
  (`AnimInstance.Montage_Pause` (`SkeletalMeshComponent.GetAnimInstance` (`self.Mesh`)) (`self.ActionMontage`)))

(fn `PlayAction`
  (params (Clip :type "AnimSequenceBase Object Reference") (Slot :type Name) (BlendIn :type "Float (double-precision)") (BlendOut :type "Float (double-precision)") (Rate :type "Float (double-precision)"))
  (returns (Length :type "Float (double-precision)"))
  (`self.StopActions` BlendOut)
  (set `self.BowClip` Clip)
  (set `self.BowShotActive` true)
  (bind _returnvalue (`AnimMontage.CreateSlotAnimationAsDynamicMontage_WithBlendSettings` Clip Slot (make `MontageBlendSettings` null (make `AlphaBlendArgs` null BlendIn)) (make `MontageBlendSettings` null (make `AlphaBlendArgs` null BlendOut)) Rate))
  (`AnimInstance.Montage_Play` (`SkeletalMeshComponent.GetAnimInstance` (`self.Mesh`)) _returnvalue Rate "MontageLength" 0.0 false)
  (set `self.ActionMontage` _returnvalue)
  (return (/ (`AnimSequenceBase.GetPlayLength` Clip) Rate)))

(fn `PlayLoop`
  (params (Clip :type "AnimSequenceBase Object Reference"))
  (bind _returnvalue (`SkeletalMeshComponent.GetAnimInstance` (`self.Mesh`)))
  (`AnimInstance.StopSlotAnimation` _returnvalue 0.2 "Base")
  (bind _returnvalue_2 (`AnimMontage.CreateSlotAnimationAsDynamicMontage_WithBlendSettings` Clip "Base" (make `MontageBlendSettings` null (make `AlphaBlendArgs` null)) (make `MontageBlendSettings` null (make `AlphaBlendArgs` null)) 1.0 100000))
  (`AnimInstance.Montage_Play` _returnvalue _returnvalue_2 1.0 "MontageLength" 0.0 false)
  (set `self.LoopMontage` _returnvalue_2))

(fn `PlayOverlay`
  (params (Clip :type "AnimSequenceBase Object Reference"))
  (returns (Length :type "Float (double-precision)"))
  (bind _returnvalue (`SkeletalMeshComponent.GetAnimInstance` (`self.Mesh`)))
  (`AnimInstance.StopSlotAnimation` _returnvalue 0.1 "Hit")
  (bind _returnvalue_2 (`AnimMontage.CreateSlotAnimationAsDynamicMontage_WithBlendSettings` Clip "Hit" (make `MontageBlendSettings` null (make `AlphaBlendArgs` null 0.05)) (make `MontageBlendSettings` null (make `AlphaBlendArgs` null 0.15))))
  (`AnimInstance.Montage_Play` _returnvalue _returnvalue_2 1.0 "MontageLength" 0.0 false)
  (return (`AnimSequenceBase.GetPlayLength` Clip)))

(fn `RemoveModule`
  (params (Module :type "SkeletalMesh Object Reference"))
  (for _array_element (`self.ArmorComponents`)
    (if (== (`SkeletalMeshComponent.GetSkeletalMeshAsset` _array_element) Module)
      (`SceneComponent.SetVisibility` _array_element false false))))

(fn `SetClipHold`
  (params (Left :type Boolean) (Right :type Boolean))
  (set `self.ClipHoldLeft` Left)
  (set `self.ClipHoldRight` Right)
  (`self.UpdateHands`))

(fn `SetDefaultModulesWorn`
  (params (Worn :type Boolean))
  (for _array_element (`self.DefaultModules`)
    (if Worn
      (`self.WearModule` _array_element)
      (else
        (`self.RemoveModule` _array_element)))))

(fn `SetFingerIdle`
  (params (Left :type Boolean) (On :type Boolean))
  (`|ExecutionSequence`
    (:`then_0`
      (if Left
        (set `self.FingerIdleLeft` On)
        (else
          (set `self.FingerIdleRight` On))))
    (:`then_1`
      (`self.UpdateHands`))))

(fn `SetFingersSuspended`
  (params (Suspended :type Boolean))
  (set `self.FingersSuspended` Suspended)
  (`self.UpdateHands`))

(fn `SetHeldBlock`
  (params (Held :type Boolean))
  (bind _asabp_undead_skeleton (cast `/Game/UndeadLegion/Blueprints/ABP_UndeadSkeleton` (`SkeletalMeshComponent.GetAnimInstance` (`self.Mesh`))))
  (`/Game/UndeadLegion/Blueprints/ABP_UndeadSkeleton.SetBlockTarget` _asabp_undead_skeleton (select `bool` Held :`true` 1.0)))

(fn `SetRootMotion`
  (params (On :type Boolean))
  (bind _returnvalue (`SkeletalMeshComponent.GetAnimInstance` (`self.Mesh`)))
  (if On
    (`AnimInstance.SetRootMotionMode` _returnvalue "RootMotionFromMontagesOnly")
    (else
      (`AnimInstance.SetRootMotionMode` _returnvalue "IgnoreRootMotion"))))

(fn `SetTwitch`
  (params (Index :type Integer) (Weight :type "Float (double-precision)"))
  (bind _asabp_undead_skeleton (cast `/Game/UndeadLegion/Blueprints/ABP_UndeadSkeleton` (`SkeletalMeshComponent.GetAnimInstance` (`self.Mesh`))))
  (`/Game/UndeadLegion/Blueprints/ABP_UndeadSkeleton.SetTwitchWeight` _asabp_undead_skeleton Index Weight))

(fn `ShowEyes`
  (params (On :type Boolean))
  (set `self.EyesVisible` On)
  (`SceneComponent.SetVisibility` (`self.EyeL`) On false)
  (`SceneComponent.SetVisibility` (`self.EyeR`) On false))

(fn `SpawnWeapon`
  (params (Index :type Integer) (Left :type Boolean))
  (bind _returnvalue (select `bool` Left :`false` (`|GetArrayItem` (`self.LoadoutRight`) Index) :`true` (`|GetArrayItem` (`self.LoadoutLeft`) Index)))
  (if (`KismetSystemLibrary.IsValidClass` _returnvalue)
    (bind _returnvalue_2 (`|SpawnActorFromClass` _returnvalue (`self.GetTransform`) "AlwaysSpawn" "SelectDefaultAtRuntime" null null))
    (`self.K2_AttachToComponent` _returnvalue_2 (`self.Mesh`) (select `bool` Left :`false` "RightHandSlot" :`true` "LeftHandSlot" :!type "Name") "SnapToTarget" "SnapToTarget" "SnapToTarget" false)
    (`KismetArrayLibrary.Array_Add` (`self.WeaponActors`) _returnvalue_2)
    (if Left
      (set `self.HasWeaponLeft` true)
      (else
        (set `self.HasWeaponRight` true)))))

(fn `StopActions`
  (params (BlendOut :type "Float (double-precision)"))
  (bind _returnvalue (`SkeletalMeshComponent.GetAnimInstance` (`self.Mesh`)))
  (set `self.BowShotActive` false)
  (`self.BowReset`)
  (`AnimInstance.Montage_Resume` _returnvalue (`self.ActionMontage`))
  (`AnimInstance.StopSlotAnimation` _returnvalue BlendOut "DefaultSlot")
  (`AnimInstance.StopSlotAnimation` _returnvalue BlendOut "UpperBody")
  (`AnimInstance.StopSlotAnimation` _returnvalue BlendOut "LeftArm")
  (`AnimInstance.StopSlotAnimation` _returnvalue BlendOut "RightArm"))

(fn `TintEyes`
  (params (Color :type "LinearColor Structure"))
  (set `self.EyeColor` Color)
  (`MeshComponent.SetVectorParameterValueOnMaterials` (`self.EyeL`) "Color" (`KismetMathLibrary.Conv_LinearColorToVector` Color))
  (`MeshComponent.SetVectorParameterValueOnMaterials` (`self.EyeR`) "Color" (`KismetMathLibrary.Conv_LinearColorToVector` Color)))

(fn `UpdateBow`
  (params (dt :type "Float (double-precision)"))
  (bind _bowmesh (`self.BowMesh`))
  (bind _returnvalue (- (`self.Draw`) (* 800.0 dt)))
  (bind _returnvalue_2 (`KismetMathLibrary.FClamp` (/ (`self.Draw`) 50.0)))
  (`PoseableMeshComponent.ResetBoneTransformByName` _bowmesh "Nock")
  (`PoseableMeshComponent.ResetBoneTransformByName` _bowmesh "Limb_U1")
  (`PoseableMeshComponent.ResetBoneTransformByName` _bowmesh "Limb_U2")
  (`PoseableMeshComponent.ResetBoneTransformByName` _bowmesh "Limb_L1")
  (`PoseableMeshComponent.ResetBoneTransformByName` _bowmesh "Limb_L2")
  (bind _returnvalue_3 (`PoseableMeshComponent.GetBoneTransformByName` _bowmesh "Brace" "WorldSpace"))
  (bind _returnvalue_4 (`KismetMathLibrary.InverseTransformLocation` _returnvalue_3 (`SceneComponent.GetSocketLocation` (`self.Mesh`) "RightHandSlot")))
  (bind _returnvalue_5 (- 0.0 (.y _returnvalue_4)))
  (bind _returnvalue_6 (* (select `bool` (`self.BowAttached`) :`true` 1.0) (* (`KismetMathLibrary.FClamp` (/ (- 50.0 (`KismetMathLibrary.Sqrt` (+ (* (.x _returnvalue_4) (.x _returnvalue_4)) (* (.z _returnvalue_4) (.z _returnvalue_4))))) 5.0)) (`KismetMathLibrary.FClamp` (/ _returnvalue_5 2.5)))))
  (bind _returnvalue_7 (* (`KismetMathLibrary.FClamp` _returnvalue_5 0.0 80.0) _returnvalue_6))
  (bind _returnvalue_8 (>= _returnvalue_7 (`self.Draw`)))
  (set `self.Draw` (select `bool` _returnvalue_8 :`false` (select `bool` (> _returnvalue _returnvalue_7) :`false` _returnvalue_7 :`true` _returnvalue) :`true` _returnvalue_7))
  (bind _returnvalue_9 (`KismetMathLibrary.MakeVector` (* (.x _returnvalue_4) _returnvalue_6) 0.0 (* (.z _returnvalue_4) _returnvalue_6)))
  (set `self.Apex` (select `bool` _returnvalue_8 :`false` (`KismetMathLibrary.VLerp` (`self.Apex`) _returnvalue_9 0.5) :`true` _returnvalue_9))
  (bind _returnvalue_10 (`PoseableMeshComponent.GetBoneTransformByName` _bowmesh "Limb_U1" "ComponentSpace"))
  (`PoseableMeshComponent.SetBoneTransformByName` _bowmesh "Limb_U1" (`KismetMathLibrary.ComposeTransforms` (`KismetMathLibrary.MakeTransform` (0.0 0.0 0.0) (`KismetMathLibrary.MakeRotator` (* -10.0 _returnvalue_2))) _returnvalue_10) "ComponentSpace")
  (bind _returnvalue_11 (`PoseableMeshComponent.GetBoneTransformByName` _bowmesh "Limb_U2" "ComponentSpace"))
  (`PoseableMeshComponent.SetBoneTransformByName` _bowmesh "Limb_U2" (`KismetMathLibrary.ComposeTransforms` (`KismetMathLibrary.MakeTransform` (0.0 0.0 0.0) (`KismetMathLibrary.MakeRotator` (* -14.0 _returnvalue_2))) _returnvalue_11) "ComponentSpace")
  (bind _returnvalue_12 (`PoseableMeshComponent.GetBoneTransformByName` _bowmesh "Limb_L1" "ComponentSpace"))
  (`PoseableMeshComponent.SetBoneTransformByName` _bowmesh "Limb_L1" (`KismetMathLibrary.ComposeTransforms` (`KismetMathLibrary.MakeTransform` (0.0 0.0 0.0) (`KismetMathLibrary.MakeRotator` (* 10.0 _returnvalue_2))) _returnvalue_12) "ComponentSpace")
  (bind _returnvalue_13 (`PoseableMeshComponent.GetBoneTransformByName` _bowmesh "Limb_L2" "ComponentSpace"))
  (`PoseableMeshComponent.SetBoneTransformByName` _bowmesh "Limb_L2" (`KismetMathLibrary.ComposeTransforms` (`KismetMathLibrary.MakeTransform` (0.0 0.0 0.0) (`KismetMathLibrary.MakeRotator` (* 14.0 _returnvalue_2))) _returnvalue_13) "ComponentSpace")
  (`PoseableMeshComponent.SetBoneLocationByName` _bowmesh "Nock" (`KismetMathLibrary.TransformLocation` _returnvalue_3 (`KismetMathLibrary.MakeVector` (.x (`self.Apex`)) (- 0.0 (`self.Draw`)) (.z (`self.Apex`)))) "WorldSpace"))

(fn `UpdateHands`
  (bind _returnvalue (or (`self.HasWeaponLeft`) (`self.ClipHoldLeft`)))
  (bind _returnvalue_2 (or (`self.HasWeaponRight`) (`self.ClipHoldRight`)))
  (bind _returnvalue_3 (not (`self.FingersSuspended`)))
  (bind _asabp_undead_skeleton (cast `/Game/UndeadLegion/Blueprints/ABP_UndeadSkeleton` (`SkeletalMeshComponent.GetAnimInstance` (`self.Mesh`))))
  (`/Game/UndeadLegion/Blueprints/ABP_UndeadSkeleton.SetHandTargets` _asabp_undead_skeleton (select `bool` _returnvalue :`true` 1.0) (select `bool` _returnvalue_2 :`true` 1.0) (select `bool` (or _returnvalue (and _returnvalue_3 (`self.FingerIdleLeft`))) :`true` 1.0) (select `bool` (or _returnvalue_2 (and _returnvalue_3 (`self.FingerIdleRight`))) :`true` 1.0)))

(fn `UserConstructionScript`
  (`self.ApplyDefaultModules`))

(fn `WearModule`
  (params (Module :type "SkeletalMesh Object Reference"))
  (for _array_element (`self.ArmorComponents`)
    (if (== (`SkeletalMeshComponent.GetSkeletalMeshAsset` _array_element) Module)
      (`SceneComponent.SetVisibility` _array_element true false)
      (return)))
  (`self.AddModuleComponent` Module))