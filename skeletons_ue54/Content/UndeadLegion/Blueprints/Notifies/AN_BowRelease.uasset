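; An animation notify that triggers the arrow release on an Undead Skeleton during a bow shot.
; It casts the mesh owner to BP_UndeadSkeleton and calls BowRelease only while a shot is active and the notifying animation's name matches the skeleton's bow clip.
; It also requires the action montage to have reached the one-second mark, with one 60 fps frame of tolerance, blocking earlier firings.
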(fn `Received_Notify`
  (params (MeshComp :type "SkeletalMeshComponent Object Reference") (Animation :type "AnimSequenceBase Object Reference") (EventReference :type "AnimNotifyEventReference Structure (by ref)"))
  (returns (ReturnValue :type Boolean))
  (bind _meshcomp (`local.MeshComp`))
  (bind _asbp_undead_skeleton (cast `/Game/UndeadLegion/Blueprints/BP_UndeadSkeleton` (`ActorComponent.GetOwner` _meshcomp))
    (:`then`
      (if (and (`/Game/UndeadLegion/Blueprints/BP_UndeadSkeleton.BowShotActive` _asbp_undead_skeleton) (and (`KismetStringLibrary.EqualEqual_StrStr` (`KismetSystemLibrary.GetObjectName` (`local.Animation`)) (`KismetSystemLibrary.GetObjectName` (`/Game/UndeadLegion/Blueprints/BP_UndeadSkeleton.BowClip` _asbp_undead_skeleton))) (>= (`AnimInstance.Montage_GetPosition` (`SkeletalMeshComponent.GetAnimInstance` _meshcomp) (`/Game/UndeadLegion/Blueprints/BP_UndeadSkeleton.ActionMontage` _asbp_undead_skeleton)) (- 1.0 0.016667))))
        (`/Game/UndeadLegion/Blueprints/BP_UndeadSkeleton.BowRelease` _asbp_undead_skeleton)
        (return false)
        (else
          (return false))))
    (:`CastFailed`
      (return false))))