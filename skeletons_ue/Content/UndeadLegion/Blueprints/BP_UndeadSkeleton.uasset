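; Modular undead skeleton with swappable armor, per-hand weapon loadouts and tintable socketed eyes.
; Armor modules are skeletal mesh components following the body through leader pose; weapons are spawned actors attached to hand slots.
; Clips play as dynamic slot montages for loops, actions and hit overlays, while ABP_UndeadSkeleton receives grip, finger, block and twitch weights.
; BeginPlay equips the start loadout, starts a loop and chains StartActions on timers.
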(event `self.ReceiveBeginPlay`
  (`self.EquipLoadout` (`self.StartLoadout`))
  (`self.PlayLoop` (`self.StartClip`))
  (`self.SetClipHold` (`self.StartHoldLeft`))
  (set `self.StartActionIndex` 0)
  (if (> (`KismetArrayLibrary.Array_Length` (`self.StartActions`)) 0)
    (`KismetSystemLibrary.K2_SetTimer` self "NextStartAction" (`self.StartActionDelay`))))

(event `self.ReceiveEndPlay`
  (params (EndPlayReason :type "EEndPlayReason Enum" :default "Destroyed"))
  (for _array_element (`self.WeaponActors`)
    (`self.K2_DestroyActor` _array_element))
  (`KismetArrayLibrary.Array_Clear` (`self.WeaponActors`)))

(fn `AddModuleComponent`
  (params (Module :type "SkeletalMesh Object Reference"))
  (bind _mesh (`self.Mesh`))
  (bind _returnvalue (`|AddComponentByClass` "/Script/Engine.SkeletalMeshComponent"))
  (`SkeletalMeshComponent.SetSkeletalMeshAsset` _returnvalue Module)
  (`SceneComponent.K2_AttachToComponent` _returnvalue _mesh "None" "SnapToTarget" "SnapToTarget" "SnapToTarget" false)
  (`SkinnedMeshComponent.SetLeaderPoseComponent` _returnvalue _mesh false false)
  (`KismetArrayLibrary.Array_Add` (`self.ArmorComponents`) _returnvalue))

(fn `ApplyDefaultModules`
  (for _array_element (`self.ArmorComponents`)
    (`ActorComponent.K2_DestroyComponent` _array_element))
  (`KismetArrayLibrary.Array_Clear` (`self.ArmorComponents`))
  (for _array_element_2 (`self.DefaultModules`)
    (`self.AddModuleComponent` _array_element_2))
  (`self.ApplyEyes`))

(fn `ApplyEyes`
  (bind _mesh (`self.Mesh`))
  (`SceneComponent.K2_AttachToComponent` (`self.EyeL`) _mesh "EyeL" "SnapToTarget" "SnapToTarget" "KeepRelative" false)
  (`SceneComponent.K2_AttachToComponent` (`self.EyeR`) _mesh "EyeR" "SnapToTarget" "SnapToTarget" "KeepRelative" false)
  (`self.ShowEyes` (`self.EyesVisible`))
  (`self.TintEyes` (`self.EyeColor`)))

(fn `EquipLoadout`
  (params (Index :type Integer))
  (for _array_element (`self.WeaponActors`)
    (`self.K2_DestroyActor` _array_element))
  (`KismetArrayLibrary.Array_Clear` (`self.WeaponActors`))
  (set `self.HasWeaponLeft` false)
  (set `self.HasWeaponRight` false)
  (set `self.CurrentLoadout` Index)
  (if (`KismetArrayLibrary.Array_IsValidIndex` (`self.LoadoutRight`) Index)
    (`self.SpawnWeapon` Index)
    (`self.SpawnWeapon` Index true))
  (`self.UpdateHands`))

(fn `GetFingerIdle`
  (params (Left :type Boolean))
  (returns (On :type Boolean))
  (return (select `bool` Left :`false` (`self.FingerIdleRight`) :`true` (`self.FingerIdleLeft`))))

(fn `GetLoadout`
  (returns (Index :type Integer))
  (return (`self.CurrentLoadout`)))

(fn `IsModuleWorn`
  (params (Module :type "SkeletalMesh Object Reference"))
  (returns (Worn :type Boolean))
  (for _array_element (`self.ArmorComponents`)
    (if (and (== (`SkeletalMeshComponent.GetSkeletalMeshAsset` _array_element) Module) (`SceneComponent.IsVisible` _array_element))
      (return true)))
  (return false))

(fn `NextStartAction`
  (bind _startactionindex (`self.StartActionIndex`))
  (if (`KismetArrayLibrary.Array_IsValidIndex` (`self.StartActions`) _startactionindex)
    (bind _length (`self.PlayAction` (`|GetArrayItem` (`self.StartActions`) _startactionindex) "DefaultSlot" 0.15 0.25 1.0))
    (`KismetSystemLibrary.PrintString` (`KismetStringLibrary.Concat_StrStr` "StartAction " (`KismetStringLibrary.Conv_IntToString` _startactionindex)) false)
    (set `self.StartActionIndex` (+ _startactionindex 1))
    (`KismetSystemLibrary.K2_SetTimer` self "NextStartAction" (+ _length (`self.StartActionGap`)))))

(fn `PauseActions`
  (`AnimInstance.Montage_Pause` (`SkeletalMeshComponent.GetAnimInstance` (`self.Mesh`)) (`self.ActionMontage`)))

(fn `PlayAction`
  (params (Clip :type "AnimSequenceBase Object Reference") (Slot :type Name) (BlendIn :type "Float (double-precision)") (BlendOut :type "Float (double-precision)") (Rate :type "Float (double-precision)"))
  (returns (Length :type "Float (double-precision)"))
  (`self.StopActions` BlendOut)
  (bind _returnvalue (`AnimMontage.CreateSlotAnimationAsDynamicMontage_WithBlendSettings` Clip Slot (make `MontageBlendSettings` null (make `AlphaBlendArgs` null BlendIn)) (make `MontageBlendSettings` null (make `AlphaBlendArgs` null BlendOut)) Rate))
  (`AnimInstance.Montage_Play` (`SkeletalMeshComponent.GetAnimInstance` (`self.Mesh`)) _returnvalue Rate "MontageLength" 0.0 false)
  (set `self.ActionMontage` _returnvalue)
  (return (/ (`AnimationAsset.GetPlayLength` Clip) Rate)))

(fn `PlayLoop`
  (params (Clip :type "AnimSequenceBase Object Reference"))
  (bind _returnvalue (`SkeletalMeshComponent.GetAnimInstance` (`self.Mesh`)))
  (`AnimInstance.StopSlotAnimation` _returnvalue 0.2 "Base")
  (bind _returnvalue_2 (`AnimMontage.CreateSlotAnimationAsDynamicMontage_WithBlendSettings` Clip "Base" (make `MontageBlendSettings` null (make `AlphaBlendArgs` null)) (make `MontageBlendSettings` null (make `AlphaBlendArgs` null)) 1.0 100000))
  (`AnimInstance.Montage_Play` _returnvalue _returnvalue_2 1.0 "MontageLength" 0.0 false)
  (set `self.LoopMontage` _returnvalue_2))

(fn `PlayOverlay`
  (params (Clip :type "AnimSequenceBase Object Reference"))
  (returns (Length :type "Float (double-precision)"))
  (bind _returnvalue (`SkeletalMeshComponent.GetAnimInstance` (`self.Mesh`)))
  (`AnimInstance.StopSlotAnimation` _returnvalue 0.1 "Hit")
  (bind _returnvalue_2 (`AnimMontage.CreateSlotAnimationAsDynamicMontage_WithBlendSettings` Clip "Hit" (make `MontageBlendSettings` null (make `AlphaBlendArgs` null 0.05)) (make `MontageBlendSettings` null (make `AlphaBlendArgs` null 0.15))))
  (`AnimInstance.Montage_Play` _returnvalue _returnvalue_2 1.0 "MontageLength" 0.0 false)
  (return (`AnimationAsset.GetPlayLength` Clip)))

(fn `RemoveModule`
  (params (Module :type "SkeletalMesh Object Reference"))
  (for _array_element (`self.ArmorComponents`)
    (if (== (`SkeletalMeshComponent.GetSkeletalMeshAsset` _array_element) Module)
      (`SceneComponent.SetVisibility` _array_element false false))))

(fn `SetClipHold`
  (params (Left :type Boolean) (Right :type Boolean))
  (set `self.ClipHoldLeft` Left)
  (set `self.ClipHoldRight` Right)
  (`self.UpdateHands`))

(fn `SetDefaultModulesWorn`
  (params (Worn :type Boolean))
  (for _array_element (`self.DefaultModules`)
    (if Worn
      (`self.WearModule` _array_element)
      (else
        (`self.RemoveModule` _array_element)))))

(fn `SetFingerIdle`
  (params (Left :type Boolean) (On :type Boolean))
  (if Left
    (set `self.FingerIdleLeft` On)
    (else
      (set `self.FingerIdleRight` On)))
  (`self.UpdateHands`))

(fn `SetFingersSuspended`
  (params (Suspended :type Boolean))
  (set `self.FingersSuspended` Suspended)
  (`self.UpdateHands`))

(fn `SetHeldBlock`
  (params (Held :type Boolean))
  (bind _asabp_undead_skeleton (cast `/Game/UndeadLegion/Blueprints/ABP_UndeadSkeleton` (`SkeletalMeshComponent.GetAnimInstance` (`self.Mesh`))))
  (`/Game/UndeadLegion/Blueprints/ABP_UndeadSkeleton.SetBlockTarget` _asabp_undead_skeleton (select `bool` Held :`false` 0.0 :`true` 1.0)))

(fn `SetRootMotion`
  (params (On :type Boolean))
  (bind _returnvalue (`SkeletalMeshComponent.GetAnimInstance` (`self.Mesh`)))
  (if On
    (`AnimInstance.SetRootMotionMode` _returnvalue "RootMotionFromEverything")
    (else
      (`AnimInstance.SetRootMotionMode` _returnvalue "IgnoreRootMotion"))))

(fn `SetTwitch`
  (params (Index :type Integer) (Weight :type "Float (double-precision)"))
  (bind _asabp_undead_skeleton (cast `/Game/UndeadLegion/Blueprints/ABP_UndeadSkeleton` (`SkeletalMeshComponent.GetAnimInstance` (`self.Mesh`))))
  (`/Game/UndeadLegion/Blueprints/ABP_UndeadSkeleton.SetTwitchWeight` _asabp_undead_skeleton Index Weight))

(fn `ShowEyes`
  (params (On :type Boolean))
  (set `self.EyesVisible` On)
  (`SceneComponent.SetVisibility` (`self.EyeL`) On false)
  (`SceneComponent.SetVisibility` (`self.EyeR`) On false))

(fn `SpawnWeapon`
  (params (Index :type Integer) (Left :type Boolean))
  (bind _returnvalue (select `bool` Left :`false` (`|GetArrayItem` (`self.LoadoutRight`) Index) :`true` (`|GetArrayItem` (`self.LoadoutLeft`) Index)))
  (if (`KismetSystemLibrary.IsValidClass` _returnvalue)
    (bind _returnvalue_2 (`|SpawnActorFromClass` _returnvalue (`self.GetTransform`) "AlwaysSpawn" "MultiplyWithRoot" null null))
    (`self.K2_AttachToComponent` _returnvalue_2 (`self.Mesh`) (`KismetStringLibrary.Conv_StringToName` (select `bool` Left :`false` "RightHandSlot" :`true` "LeftHandSlot")) "SnapToTarget" "SnapToTarget" "SnapToTarget" false)
    (`KismetArrayLibrary.Array_Add` (`self.WeaponActors`) _returnvalue_2)
    (if Left
      (set `self.HasWeaponLeft` true)
      (else
        (set `self.HasWeaponRight` true)))))

(fn `StopActions`
  (params (BlendOut :type "Float (double-precision)"))
  (bind _returnvalue (`SkeletalMeshComponent.GetAnimInstance` (`self.Mesh`)))
  (`AnimInstance.StopSlotAnimation` _returnvalue BlendOut "DefaultSlot")
  (`AnimInstance.StopSlotAnimation` _returnvalue BlendOut "UpperBody")
  (`AnimInstance.StopSlotAnimation` _returnvalue BlendOut "LeftArm")
  (`AnimInstance.StopSlotAnimation` _returnvalue BlendOut "RightArm"))

(fn `TintEyes`
  (params (Color :type "LinearColor Structure"))
  (set `self.EyeColor` Color)
  (`MeshComponent.SetColorParameterValueOnMaterials` (`self.EyeL`) "Color" Color)
  (`MeshComponent.SetColorParameterValueOnMaterials` (`self.EyeR`) "Color" Color))

(fn `UpdateHands`
  (bind _returnvalue (not (`self.FingersSuspended`)))
  (bind _returnvalue_2 (or (`self.HasWeaponLeft`) (`self.ClipHoldLeft`)))
  (bind _returnvalue_3 (or (`self.HasWeaponRight`) (`self.ClipHoldRight`)))
  (bind _asabp_undead_skeleton (cast `/Game/UndeadLegion/Blueprints/ABP_UndeadSkeleton` (`SkeletalMeshComponent.GetAnimInstance` (`self.Mesh`))))
  (`/Game/UndeadLegion/Blueprints/ABP_UndeadSkeleton.SetHandTargets` _asabp_undead_skeleton (select `bool` _returnvalue_2 :`false` 0.0 :`true` 1.0) (select `bool` _returnvalue_3 :`false` 0.0 :`true` 1.0) (select `bool` (or _returnvalue_2 (and _returnvalue (`self.FingerIdleLeft`))) :`false` 0.0 :`true` 1.0) (select `bool` (or _returnvalue_3 (and _returnvalue (`self.FingerIdleRight`))) :`false` 0.0 :`true` 1.0)))

(fn `UserConstructionScript`
  (`self.ApplyDefaultModules`))

(fn `WearModule`
  (params (Module :type "SkeletalMesh Object Reference"))
  (for _array_element (`self.ArmorComponents`)
    (if (== (`SkeletalMeshComponent.GetSkeletalMeshAsset` _array_element) Module)
      (`SceneComponent.SetVisibility` _array_element true false)))
  (`self.AddModuleComponent` Module))